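; BP_Square is a Level 1 actor that jumps between two hard-coded world positions when something overlaps its Box trigger.
; On overlap it snaps along Y to a distant spot, waits briefly, then sets a second position with sweep enabled so blocking collision can stop it.
; Leftover Cube offset nodes are disconnected, and RunAwayFunction and the construction script are empty.
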(event OnComponentBeginOverlap(Box)
  (params (OverlappedComponent :type Primitive%20Component%20Object%20Reference) (OtherActor :type Actor%20Object%20Reference) (OtherComp :type Primitive%20Component%20Object%20Reference) (OtherBodyIndex :type Integer) (bFromSweep :type Boolean) (SweepResult :type Hit%20Result%20Structure%20%28by%20ref%29))
  (Transformation|SetActorLocation "-340.000000,-1000.000000,0.000000" false false)
  (Utilities|FlowControl|Delay 0.9)
  (Transformation|SetActorLocation "-340.000000,180.000000,0.000000" true false))

(fn ConstructionScript)

(fn RunAwayFunction)