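; BP_SmallSphere is a short-lived drifting sphere that adds to the score in BP_BadBotGamemode when the character, a default pawn or a bot pawn overlaps it.
; Tick moves SphereVolume along its forward vector and spins SphereMesh by a random rotation set on BeginPlay.
; After a delay, a timeline scales it in.
; Overlap or a lifetime timer triggers a guarded WinkOut timeline that rescales and destroys it.
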(event Custom|WinkIn
  ;[0.6042 0.08392 0.07237] WinkIn Timeline
  (bind _scale (Timeline|WinkINTimeleine Play)
    (:Update
      (Transformation|SetWorldScale3D (Variables|Default|GetSphereMesh) _scale))))

(event Custom|WinkOut
  ;[0.6042 0.08392 0.07237] WinkOut Timeline
  ;;[0.15 0.15 0.15 0.5] So its not winking out while aready winking out due to collision
  (if (not (Variables|Default|GetIsWinking?))
    (Variables|Default|SetIsWinking? true)
    (bind _scale (Timeline|WinkOutTimeline Play)
      (:Update
        (Transformation|SetWorldScale3D (Variables|Default|GetSphereMesh) (Math|Conversions|ToVector(Float) _scale)))
      (:Finished
        (Actor|DestroyActor)))))

(event Custom|OnSphereOverlap
  (params (OverlappedComponent :type Primitive%20Component%20Object%20Reference) (OtherActor :type Actor%20Object%20Reference) (OtherComp :type Primitive%20Component%20Object%20Reference) (OtherBodyIndex :type Integer) (bFromSweep :type Boolean) (SweepResult :type Hit%20Result%20Structure%20%28by%20ref%29))
  ;[0.6042 0.08392 0.07237] Handle overlap + scoring
  (if (Math|Boolean|ORBoolean (Class|GameplayStatics|ObjectIsA OtherActor "/Game/ThirdPerson/Blueprints/BP_ThirdPersonCharacter.BP_ThirdPersonCharacter_C") (Class|GameplayStatics|ObjectIsA OtherActor "/Script/Engine.DefaultPawn") (Class|GameplayStatics|ObjectIsA OtherActor "/Game/Levels/Level_1/Blueprints/BotPawn/BP_BotPawn.BP_BotPawn_C"))
    (bind _asbp_bad_bot_gamemode (Utilities|Casting|CastToBP_BadBotGamemode (Game|GetGameMode)))
    (Default|IncrementScore _asbp_bad_bot_gamemode)
    (CallFunction|WinkOut)))

(event EventTick
  (params (DeltaSeconds :type Float%20%28single-precision%29))
  (bind _outputpin (CallFunction|UpdateLocation DeltaSeconds DeltaSeconds))
  (CallFunction|UpdateRotation _outputpin)
  ;[0.6042 0.08392 0.07237] Handle overlap + scoring
  (Collision|AssignOnComponentBeginOverlap (Variables|Default|GetSphereVolume) (delegate Custom|OnSphereOverlap)))

(event EventBeginPlay
  (Utilities|FlowControl|Delay 2.0)
  (CallFunction|Winkin)
  (CallFunction|InitializeDeltaRotation)
  ;[0.6042 0.08392 0.07237] WinkOut Timeline
  (Utilities|Time|SetTimerbyEvent (delegate Custom|WinkOut) (Variables|Default|GetLifeTime))
  ;[0.6042 0.08392 0.07237] Handle overlap + scoring
  (Collision|AssignOnComponentBeginOverlap (Variables|Default|GetSphereVolume) (delegate Custom|OnSphereOverlap)))

(fn ConstructionScript)

(fn SpeedVector
  (params (Time :type Float%20%28double-precision%29))
  (return "0, 0, 0"))

(fn BubbleMoving
  (params (InputPin :type Float%20%28single-precision%29) (A :type Float%20%28double-precision%29))
  (Transformation|AddWorldOffset (Variables|Default|GetSphereMesh) (* (Math|Vector|GetForwardVector (Variables|Default|GetSphereMesh)) (* A (Variables|Default|GetTimeMove))) false false)
  (Transformation|AddWorldRotation (Variables|Default|GetSphereMesh) (* (Variables|Default|GetDeltaRotation) InputPin) false false))

(fn InitializeDeltaRotation
  (Variables|Default|SetDeltaRotation (* (Math|Random|RandomRotator false) (Variables|Default|GetRandomRotationFactor))))

(fn UpdateLocation
  (params (Delta%20Seconds :type Float%20%28double-precision%29) (InputPin :type Float%20%28single-precision%29))
  (Transformation|AddWorldOffset (Variables|Default|GetSphereVolume) (* (Math|Vector|GetForwardVector (Variables|Default|GetSphereVolume)) (* Delta%20Seconds (Variables|Default|GetTimeMove))) false false)
  (return InputPin))

(fn UpdateRotation
  (params (DeltaSeconds :type Float%20%28single-precision%29))
  (Transformation|AddWorldRotation (Variables|Default|GetSphereMesh) (* (Variables|Default|GetDeltaRotation) DeltaSeconds) false false))