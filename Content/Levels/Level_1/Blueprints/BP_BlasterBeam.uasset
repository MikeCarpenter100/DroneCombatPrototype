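; BP_BlasterBeam is a blaster beam actor that damages what it hits and then destroys itself.
; BeginPlay binds the BeamMesh hit event to HandleOnHit, which spawns a Niagara burst aligned to the impact normal.
; Actors implementing BPI_Damageable receive GetHurtMessage with the Damage value.
; An unconnected branch that quits the game when TargetPawn is hit remains in HandleOnHit but never runs.
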(event Custom|OnComponentHit_Event
  (params (HitComponent :type Primitive%20Component%20Object%20Reference) (OtherActor :type Actor%20Object%20Reference) (OtherComp :type Primitive%20Component%20Object%20Reference) (NormalImpulse :type Vector) (Hit :type Hit%20Result%20Structure%20%28by%20ref%29))
  (CallFunction|HandleonHit OtherActor Hit))

(event EventBeginPlay
  (Collision|AssignOnComponentHit (Variables|Default|GetBeamMesh) (delegate Custom|OnComponentHit_Event)))

(fn ConstructionScript)

(fn HandleonHit
  (params (Hit%20Actor :type Object%20Object%20Reference) (Hit :type Hit%20Result%20Structure%20%28by%20ref%29))
  (bind (_bblockinghit _binitialoverlap _time _distance _location _impactpoint _normal) (Collision|BreakHitResult Hit))
  (Niagara|SpawnSystematLocation "/Game/Levels/Level_1/Niagra/NS_Beam_Burst.NS_Beam_Burst" _location (Math|Conversions|RotationFromXVector _normal))
  (if (Utilities|DoesObjectImplementInterface Hit%20Actor "/Game/Levels/Level_1/Blueprints/Interfaces/BPI_Damageable.BPI_Damageable_C")
    (Class|BPIDamageable|GetHurt(Message) Hit%20Actor (Variables|Default|GetDamage)))
  (Actor|DestroyActor))