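; BP_SphereSpawner is a level actor that repeatedly spawns BP_SmallSphere actors around itself.
; A looping timer set on BeginPlay fires SpawnSphere every SpawnTime, giving each sphere a random rotation.
; Spawn points combine a random direction with a random distance up to SpawnRadius, so they cluster toward the center rather than filling the volume evenly.
; A debug sphere draw of the radius is left unconnected.
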(event Custom|SpawnSphere
  (Game|SpawnActorfromClass "/Game/Levels/Level_1/Blueprints/BP_SmallSphere.BP_SmallSphere_C" (Math|Transform|MakeTransform (CallFunction|GetRandomPointInsphereRadius) (Math|Random|RandomRotator false) "1.000000,1.000000,1.000000") "Undefined" "MultiplyWithRoot" 0 0))

(event EventBeginPlay
  (Utilities|Time|SetTimerbyEvent (delegate Custom|SpawnSphere) (Variables|Default|GetSpawnTime) true))

(event EventTick
  (params (DeltaSeconds :type Float%20%28single-precision%29)))

(fn ConstructionScript)

(fn GetRandomPointInsphereRadius
  (return (+ (Transformation|GetActorLocation) (* (Math|Vector|GetForwardVector (Math|Random|RandomRotator false)) (Math|Random|RandomFloatinRange 0.0 (Variables|Default|GetSpawnRadius))))))