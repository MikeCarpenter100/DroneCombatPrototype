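; BP_Arrower is a turret-style actor that fires BP_Arrow_Damage arrows at an enemy cube.
; On BeginPlay it stores the first BP_Enemy_Cube found and, if one exists, starts a looping timer set by ShootingSpeed.
; Each timer firing spawns an arrow at the mesh's S_Rifle socket.
; Tick snaps rotation toward the cube without a validity check, leaving the smoothed RInterpTo unused.
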(event Custom|Arrows_Shooting
  ;[0.15 0.15 0.15 0.5] Shooting arrows from Arrower
  (Game|SpawnActorfromClass "/Game/Levels/Testing_Level/BP/BP_Arrow_Damage.BP_Arrow_Damage_C" (Transformation|GetSocketTransform (Variables|Default|GetSM_Arrower) "S_Rifle" "RTS_World") "Undefined" "MultiplyWithRoot" 0 0))

(event EventBeginPlay
  ;[0.15 0.15 0.15 0.5] Shooting arrows from Arrower
  ;[0.15 0.15 0.15 0.5] Target of arrows
  (bind _outactors (Actor|GetAllActorsOfClass "/Game/Levels/Testing_Level/BP/BP_Enemy_Cube.BP_Enemy_Cube_C"))
  (if (Utilities|Array|IsValidIndex _outactors)
    (Variables|Default|SetEnemy%20Cube (Utilities|Array|Get(acopy) _outactors))
    (Utilities|Time|SetTimerbyEvent (delegate Custom|Arrows_Shooting) (Variables|Default|GetShooting_Speed) true)))

(event EventTick
  (params (DeltaSeconds :type Float%20%28single-precision%29))
  (Transformation|SetActorRotation (Math|Rotator|FindLookatRotation (Transformation|GetActorLocation) (Transformation|GetActorLocation (Variables|Default|GetEnemy%20Cube)))))

(fn ConstructionScript)